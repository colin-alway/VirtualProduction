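; BP_Patch is a cube actor whose color shifts hue each time its CallMe function runs.
; The construction script gives the Cube a dynamic instance of M_Actor and stores it as DynamicMaterial.
; CallMe prints the current BaseColor, then advances its hue through an RGB-to-HSV round trip.
; BeginPlay and Tick do nothing, as an older timed hue cycle and material setup remain unwired in the event graph.
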(event EventBeginPlay)

(event Collision|EventActorBeginOverlap
  (params (OtherActor :type Actor%20Object%20Reference)))

(event EventTick
  (params (DeltaSeconds :type Float%20%28single-precision%29)))

(fn ConstructionScript
  (bind _returnvalue (Rendering|Material|CreateDynamicMaterialInstance (Variables|Default|GetCube) 0 "/Game/VprodProject/Materials/M_Actor.M_Actor" "None" :!class /Script/Engine.PrimitiveComponent))
  (Variables|Default|SetDynamicMaterial _returnvalue))

(fn CallMe
  (bind _returnvalue (Rendering|Material|GetVectorParameterValue (Variables|Default|GetDynamicMaterial) "BaseColor" :!class /Script/Engine.MaterialInstanceDynamic))
  (Development|PrintString (Utilities|String|ToString(Integer) _returnvalue))
  (Rendering|Material|SetVectorParameterValue (Variables|Default|GetDynamicMaterial) "BaseColor" (Class|KismetMathLibrary|HSVtoRGBVector (Utilities|Struct|MakeLinearColor (+ (.r (Class|KismetMathLibrary|RGBtoHSVVector _returnvalue)) 15.0) (.g (Class|KismetMathLibrary|RGBtoHSVVector _returnvalue)) (.b (Class|KismetMathLibrary|RGBtoHSVVector _returnvalue)) (.a (Class|KismetMathLibrary|RGBtoHSVVector _returnvalue)))) :!class /Script/Engine.MaterialInstanceDynamic))