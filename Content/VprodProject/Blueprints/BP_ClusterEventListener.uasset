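; BP_ClusterEventListener is an nDisplay debug actor that receives cluster events and prints their contents.
; It registers itself with the cluster API as an event listener on BeginPlay and removes itself on EndPlay.
; Each JSON cluster event is printed with its name, type, category, and joined parameter keys and values.
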(event EventBeginPlay
  (Class|DisplayClusterBlueprintAPI|AddClusterEventListener (Class|DisplayClusterBlueprintLib|GetAPI) self)
  (Development|PrintString "### add cluster event listener"))

(event Collision|EventActorBeginOverlap
  (params (OtherActor :type Actor%20Object%20Reference)))

(event EventTick
  (params (DeltaSeconds :type Float%20%28single-precision%29)))

(event EventEndPlay
  (params (EndPlayReason :type EEndPlayReason%20Enum :default "Destroyed"))
  (Class|DisplayClusterBlueprintAPI|RemoveClusterEventListener (Class|DisplayClusterBlueprintLib|GetAPI) self))

(event EventOnClusterEventJson
  (params (Event :type Display%20Cluster%20Cluster%20Event%20Json%20Structure%20%28by%20ref%29))
  (bind (_name _type _category _parameters) (Utilities|Struct|BreakDisplayClusterClusterEventJson Event))
  (bind _keys (Utilities|Map|Keys _parameters))
  (bind _values (Utilities|Map|Values _parameters))
  (Development|PrintText (Utilities|Text|FormatText "### Name={A} Type={B} Category={C} Keys={D} Values={E}" _name _type _category (Utilities|String|JoinStringArray _keys "==") (Utilities|String|JoinStringArray _values "=="))))

(fn ConstructionScript)