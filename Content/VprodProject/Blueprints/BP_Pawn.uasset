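; Pawn for an nDisplay project that wires a main UI to a spawned BP_Patch actor and monitors cluster events.
; On BeginPlay it shows the mouse cursor to avoid nDisplay capture, spawns the patch, adds WBP_Main and binds its button to the patch's CallMe.
; It registers as a cluster event listener until EndPlay, writing timestamped details of JSON events not named Node_0 to the UI.
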(event Custom|OnClicked_Event
  (Default|CallMe (Variables|Default|GetPatch)))

(event Collision|EventActorBeginOverlap
  (params (OtherActor :type Actor%20Object%20Reference)))

(event EventTick
  (params (DeltaSeconds :type Float%20%28single-precision%29)))

(event EventEndPlay
  (params (EndPlayReason :type EEndPlayReason%20Enum :default "Destroyed"))
  (Class|DisplayClusterBlueprintAPI|RemoveClusterEventListener (Class|DisplayClusterBlueprintLib|GetAPI) self))

(event EventBeginPlay
  ;[1 1 1] moved from Ndisplay level blueprint
  (Utilities|FlowControl|Sequence
    (:then_0
      ;[1 1 1] prevents nDisplay capturing mouse
      (Variables|/Script/Engine.PlayerController|SetbShowMouseCursor (Game|GetPlayerController 0) true))
    (:then_1
      (bind _returnvalue (Game|SpawnActorfromClass "/Game/VprodProject/Blueprints/BP_Patch.BP_Patch_C" (Math|Transform|MakeTransform "0.000000,-150.000000,80.000000") "Undefined" 0 0))
      (Variables|Default|SetPatch _returnvalue)
      (bind _returnvalue_2 (Game|ConstructObjectfromClass "/Game/VprodProject/Blueprints/WBP_Main.WBP_Main_C"))
      (bind _output_get (Variables|Default|SetUI _returnvalue_2))
      (UserInterface|Viewport|AddtoViewport _output_get 0)
      (EventDispatchers|AssignOnClicked (Variables|/Game/VprodProject/Blueprints/WBP_Main.WBP_Main_C|GetButton _output_get) (delegate Custom|OnClicked_Event)))
    (:then_2
      (Class|DisplayClusterBlueprintAPI|AddClusterEventListener (Class|DisplayClusterBlueprintLib|GetAPI) self))))

(event EventOnClusterEventJson
  (params (Event :type Display%20Cluster%20Cluster%20Event%20Json%20Structure%20%28by%20ref%29))
  (bind (_name _type _category) (Utilities|Struct|BreakDisplayClusterClusterEventJson Event))
  (bind _returnvalue (Math|DateTime|Now))
  (bind (_year _month _day _hour _minute _second _millisecond) (Math|DateTime|BreakDateTime _returnvalue))
  (if (Utilities|Enum|NotEqual(Enum) _name "Node_0")
    (Rendering|Components|TextRender|SetText (Variables|/Game/VprodProject/Blueprints/WBP_Main.WBP_Main_C|GetListener (Variables|Default|GetUI)) (Utilities|Text|FormatText "Time={A}:{B}:{C} 
Name={D} 
Type={E} 
Category={F}" _minute _second _millisecond _name _type _category))))

(fn ConstructionScript)